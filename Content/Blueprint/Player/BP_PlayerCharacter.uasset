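; Networked player character for a fighting game with a shared camera, where each player turns to face the other while moving.
; Remote clients add input mapping, view through BP_SharedCamera, and flip walk directions by their side of that camera.
; Input sets an animation state, gated by falling and a kick lock.
; A looping timer turns state changes into montages, relayed through PlayAnimMontageOnServer to PlayAnimMontageOnClient.
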(event `self.ReceiveBeginPlay`
  (`/Engine/EditorBlueprintResources/ActorMacros.Switch Has Authority`
    (:`Remote`
      (bind _asplayer_controller (cast `PlayerController` (`self.GetController`)))
      (`EnhancedInputSubsystemInterface.AddMappingContext` (pcsubsystem `EnhancedInputLocalPlayerSubsystem` _asplayer_controller) "/Game/Inputs/IMC_Player.IMC_Player" 1 (struct))
      (bind _returnvalue (`GameplayStatics.GetActorOfClass` "/Game/Blueprint/SharedCamera/BP_SharedCamera.BP_SharedCamera_C"))
      (set `self.SharedCamera` _returnvalue)
      (bind _asplayer_controller_2 (cast `PlayerController` (`self.GetController`)))
      (`PlayerController.SetViewTargetWithBlend` _asplayer_controller_2 _returnvalue 0.0 "VTBlend_Linear" 0.0 false)
      (`KismetSystemLibrary.K2_SetTimerDelegate` (delegate `UpdateAnimation`) 0.1 true))))

(event `UpdateAnimation`
  (switch `/Game/Blueprint/Player/AnimState` (`self.AnimState`)
    (:`NewEnumerator0`
      (if (not (`|EnumEquality` (`self.PlayingAnim`) "NewEnumerator0"))
        (set `self.PlayingAnim` "NewEnumerator0")
        (`self.Play Anim Montage On Server` "/Game/Assets/Characters/Animation/Fighting_Idle_Montage.Fighting_Idle_Montage")))
    (:`NewEnumerator1`
      (if (not (`|EnumEquality` (`self.PlayingAnim`) "NewEnumerator1"))
        (set `self.PlayingAnim` "NewEnumerator1")
        (`self.Play Anim Montage On Server` "/Game/Assets/Characters/Ninja/Standing_Walk_Forward_Anim_Montage.Standing_Walk_Forward_Anim_Montage")))
    (:`NewEnumerator2`
      (if (not (`|EnumEquality` (`self.PlayingAnim`) "NewEnumerator2"))
        (set `self.PlayingAnim` "NewEnumerator2")
        (`self.Play Anim Montage On Server` "/Game/Assets/Characters/Ninja/Crouch_Walk_Back_Montage.Crouch_Walk_Back_Montage")))
    (:`NewEnumerator3`
      (if (not (`|EnumEquality` (`self.PlayingAnim`) "NewEnumerator3"))
        (set `self.PlayingAnim` "NewEnumerator3")
        (`self.Play Anim Montage On Server` "/Game/Assets/Characters/Animation/Fall_A_Loop_Montage.Fall_A_Loop_Montage")))
    (:`NewEnumerator4`
      (if (not (`|EnumEquality` (`self.PlayingAnim`) "NewEnumerator4"))
        (set `self.PlayingAnim` "NewEnumerator4")
        (`self.Play Anim Montage On Server` "/Game/Assets/Characters/Animation/Inside_Crescent_Kick_Montage.Inside_Crescent_Kick_Montage")))))

(event `EnhancedInput|/Game/Inputs/Walk`
  (params (ActionValue :type "Float (double-precision)") (ElapsedSeconds :type "Float (double-precision)") (TriggeredSeconds :type "Float (double-precision)") (InputAction :type "InputAction Object Reference" :default "/Game/Inputs/Walk.Walk"))
  (bind _sharedcamera (`self.SharedCamera`))
  (bind _returnvalue (`KismetMathLibrary.Conv_RotatorToVector` (`self.K2_GetActorRotation`)))
  (:`Triggered`
    (`|ExecutionSequence`
      (:`then_0`
        (if (`self.IsOnTheRight`)
          (`self.AddMovementInput` _returnvalue ActionValue)
          (if (> ActionValue 0.0)
            (`self.SetAnimationState` "NewEnumerator1" :!label _label)
            (else
              (`self.SetAnimationState` "NewEnumerator2" :!label _label_2)))
          (else
            (`self.AddMovementInput` (* _returnvalue -1.0) ActionValue)
            (if (> ActionValue 0.0)
              (goto _label_2)
              (else
                (goto _label))))))
      (:`then_1`
        (`self.UpdateRotation`))))
  (:`Started`
    (if (> (`KismetMathLibrary.Dot_VectorVector` (- (`self.K2_GetActorLocation` _sharedcamera) (`self.K2_GetActorLocation`)) (`SceneComponent.GetRightVector` (`/Game/Blueprint/SharedCamera/BP_SharedCamera.Camera` _sharedcamera))) 0.0)
      (set `self.IsOnTheRight` true)
      (else
        (set `self.IsOnTheRight` false))))
  (:`Completed`
    (`self.SetAnimationState` "NewEnumerator0")))

(event `EnhancedInput|/Game/Inputs/WalkSide`
  (params (ActionValue :type "Float (double-precision)") (ElapsedSeconds :type "Float (double-precision)") (TriggeredSeconds :type "Float (double-precision)") (InputAction :type "InputAction Object Reference" :default "/Game/Inputs/WalkSide.WalkSide"))
  (bind _returnvalue (`self.GetActorRightVector`))
  (bind _sharedcamera (`self.SharedCamera`))
  (:`Triggered`
    (`|ExecutionSequence`
      (:`then_0`
        (if (`self.IsOnTheRight`)
          (`self.AddMovementInput` (* _returnvalue -1.0) ActionValue)
          (else
            (`self.AddMovementInput` _returnvalue ActionValue))))
      (:`then_1`
        (`self.UpdateRotation`))))
  (:`Started`
    (if (> (`KismetMathLibrary.Dot_VectorVector` (- (`self.K2_GetActorLocation` _sharedcamera) (`self.K2_GetActorLocation`)) (`SceneComponent.GetRightVector` (`/Game/Blueprint/SharedCamera/BP_SharedCamera.Camera` _sharedcamera))) 0.0)
      (set `self.IsOnTheRight` true)
      (else
        (set `self.IsOnTheRight` false)))))

(event `UpdateRotation`
  (bind _outactors (`GameplayStatics.GetAllActorsOfClass` "BP_PlayerCharacter_C"))
  (for _array_element _outactors
    (if (!= _array_element self)
      (`Controller.SetControlRotation` (`self.GetController`) (`KismetMathLibrary.FindLookAtRotation` (`self.K2_GetActorLocation`) (`self.K2_GetActorLocation` _array_element))))))

(event `EnhancedInput|/Game/Inputs/Jump`
  (params (ActionValue :type Boolean) (ElapsedSeconds :type "Float (double-precision)") (TriggeredSeconds :type "Float (double-precision)") (InputAction :type "InputAction Object Reference" :default "/Game/Inputs/Jump.Jump"))
  (:`Started`
    (`self.Jump`)
    (`KismetSystemLibrary.DelayUntilNextTick`)
    (`self.SetAnimationState` "NewEnumerator3")))

(event `EnhancedInput|/Game/Inputs/Kick`
  (params (ActionValue :type Boolean) (ElapsedSeconds :type "Float (double-precision)") (TriggeredSeconds :type "Float (double-precision)") (InputAction :type "InputAction Object Reference" :default "/Game/Inputs/Kick.Kick"))
  (:`Started`
    (`self.SetAnimationState` "NewEnumerator4")
    (`KismetSystemLibrary.Delay` 1.0)
    (set `self.AnimState` "NewEnumerator0")))

(event `Play Anim Montage On Server`
  (params (AnimMontage :type "AnimMontage Object Reference"))
  (`self.Play Anim Montage On Client` AnimMontage))

(event `Play Anim Montage On Client`
  (params (AnimMontage :type "AnimMontage Object Reference"))
  (`self.PlayAnimMontage` AnimMontage))

(fn `SetAnimationState`
  (params (Anim :type "/Game/Blueprint/Player/AnimState Enum" :default "NewEnumerator0"))
  (locals (AnimLocal :type "/Game/Blueprint/Player/AnimState Enum"))
  (set `local.AnimLocal` Anim)
  (if (`|EnumEquality` (`self.AnimState`) "NewEnumerator4")
    _
    (elif (`NavMovementInterface.IsFalling` (`self.CharacterMovement`))
      (switch `/Game/Blueprint/Player/AnimState` (`local.AnimLocal`)
        (:`NewEnumerator3`
          (set `self.AnimState` (`local.AnimLocal`)))
        (:`NewEnumerator4`
          (set `self.AnimState` (`local.AnimLocal`))))
      (else
        (switch `/Game/Blueprint/Player/AnimState` (`local.AnimLocal`)
          (:`NewEnumerator0`
            (set `self.AnimState` (`local.AnimLocal`) :!label _label))
          (:`NewEnumerator1`
            (goto _label))
          (:`NewEnumerator2`
            (goto _label))
          (:`NewEnumerator4`
            (set `self.AnimState` (`local.AnimLocal`))))))))

(fn `UserConstructionScript`)