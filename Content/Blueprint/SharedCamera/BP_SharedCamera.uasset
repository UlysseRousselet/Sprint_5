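; BP_SharedCamera is a shared camera actor that keeps two player characters framed together.
; On BeginPlay, only the non-authority (Remote) side polls with a retriggerable delay until exactly two BP_PlayerCharacter actors exist, then stores them in PlayerList.
; Each Tick offsets it horizontally from their midpoint, perpendicular to the line between them and scaled by their separation, then rotates it to face that midpoint.
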(event `self.ReceiveBeginPlay`
  (`/Engine/EditorBlueprintResources/ActorMacros.Switch Has Authority`
    (:`Remote`
      (bind _outactors (`GameplayStatics.GetAllActorsOfClass` "/Game/Blueprint/Player/BP_PlayerCharacter.BP_PlayerCharacter_C" :!label _label))
      (if (== (`KismetArrayLibrary.Array_Length` _outactors) 2)
        (set `self.PlayerList` _outactors)
        (else
          (`KismetSystemLibrary.RetriggerableDelay` 0.2)
          (goto _label))))))

(event `self.ReceiveTick`
  (params (DeltaSeconds :type "Float (single-precision)"))
  (bind _output (`|GetArrayItem` (`self.PlayerList`)))
  (bind _output_2 (`|GetArrayItem` (`self.PlayerList`) 1))
  (bind _returnvalue (`KismetMathLibrary.VLerp` (`self.K2_GetActorLocation` _output) (`self.K2_GetActorLocation` _output_2) 0.5))
  (`/Engine/EditorBlueprintResources/StandardMacros.IsValid` _output
    (:`Is Valid`
      (`/Engine/EditorBlueprintResources/StandardMacros.IsValid` _output_2
        (:`Is Valid`
          (`self.K2_SetActorLocation` (+ (* (`KismetMathLibrary.Cross_VectorVector` (`KismetMathLibrary.Normal` (- (`self.K2_GetActorLocation` _output_2) (`self.K2_GetActorLocation` _output))) (`KismetMathLibrary.Vector_Up`)) (`KismetMathLibrary.Vector_Distance` (`self.K2_GetActorLocation` _output_2) (`self.K2_GetActorLocation` _output))) _returnvalue))
          (`self.K2_SetActorRotation` (`KismetMathLibrary.FindLookAtRotation` (`self.K2_GetActorLocation`) _returnvalue)))))))

(fn `OnRep_PlayerList`)

(fn `UserConstructionScript`)